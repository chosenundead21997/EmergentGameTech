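; BP_Phone is the phone-side Blueprint that sets up a player's UI-driven interface when play begins.
; BeginPlay creates and displays WBP_Interface, calls the ESpawned event, then shows the mouse cursor and locks input to UI-only on that widget.
; It also prints a debug message when running without authority.
; Disconnected leftover nodes would create an OSC client and send a test message to a hardcoded IP, but never run.
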(event EventBeginPlay
  (Utilities|FlowControl|Sequence
    (:then_0
      (bind _returnvalue (UserInterface|CreateWidget "/Game/AppStuff/WBP_Interface.WBP_Interface_C"))
      (Variables|Default|SetHUDRef _returnvalue)
      (UserInterface|Viewport|AddtoViewport _returnvalue 0)
      (Default|CallESpawned))
    (:then_1
      (Variables|/Script/Engine.PlayerController|SetbShowMouseCursor (Game|GetPlayerController 0) true)
      (Input|SetInputModeUIOnly (Game|GetPlayerController 0) (Variables|Default|GetHUDRef) "LockAlways" false))
    (:then_2
      (Networking|SwitchHasAuthority
        (:Remote
          (Development|PrintString (Utilities|String|Append (Utilities|GetDisplayName self) " is remote")))))))

(event Input|KeyboardEvents|DebugKeyF
  (params (Key :type Key%20Structure :default "None") (ActionValue :type Input%20Action%20Value%20Structure)))

(fn ConstructionScript)