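; Game mode for a companion app that starts a LAN session on BeginPlay and tracks connecting players.
; PostLogin adds each new player controller to a list, whose names Tick prints every frame as debug output.
; An OSC handler prints incoming message addresses, but the server creation and binding are disconnected, as are host-versus-client authority debug checks.
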(event `self.ReceiveTick`
  (params (DeltaSeconds :type "Float (single-precision)"))
  (for _array_element (`self.In Controller`)
    (`KismetSystemLibrary.PrintString` (`KismetSystemLibrary.GetDisplayName` _array_element))))

(event `self.K2_PostLogin`
  (params (NewPlayer :type "PlayerController Object Reference"))
  (`parent.K2_PostLogin` NewPlayer)
  (`KismetArrayLibrary.Array_Add` (`self.In Controller`) NewPlayer))

(event `self.HandleStartingNewPlayer`
  (params (NewPlayer :type "PlayerController Object Reference")))

(event `self.ReceiveBeginPlay`
  (`CreateSessionCallbackProxy.CreateSession` (`GameplayStatics.GetPlayerController` 0) 0 true false
    (:`OnSuccess`
      (`KismetSystemLibrary.PrintString` "Hello"))))

(event `OSCMessageReceived`
  (params (Message :type "OSCMessage Structure (by ref)") (IPAddress :type String) (Port :type Integer))
  (`KismetSystemLibrary.PrintString` "Hello")
  (bind _returnvalue (`OSCManager.GetOSCMessageAddress` Message))
  (bind _returnvalue_2 (`OSCManager.GetOSCAddressFullPath` _returnvalue))
  (`KismetSystemLibrary.PrintString` _returnvalue_2))

(fn `UserConstructionScript`)